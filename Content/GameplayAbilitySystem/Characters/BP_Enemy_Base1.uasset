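; Base enemy character using the Gameplay Ability System, with sword combat and a floating health bar.
; On BeginPlay it initializes the health widget, grants equip and attack abilities, sends a sword equip event and adds the enemy tag, all gated on the widget cast.
; Tick turns the health bar toward the player's camera.
; An UpdateState event stores the Chasing, Strafing or Attacking state and adjusts walk speed to match.
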(event EventBeginPlay
  (bind _asw_enemy_health (Utilities|Casting|CastToW_EnemyHealth (UserInterface|GetWidget (Variables|Default|GetHealth%20Bar%20Widget%20Component)))
    (:then
      (Variables|/Game/UI/Widgets/W_EnemyHealth.W_EnemyHealth_C|SetOwning%20Enemy _asw_enemy_health self)
      (Default|Initialize _asw_enemy_health)
      (CallFunction|GiveAbilities)
      (Ability|SendGameplayEventtoActor self "(TagName=\"Event.Weapon.Equip\")" (Utilities|Struct|MakeGameplayEventData "(GameplayTags=((TagName=\"Weapon.Melee.Sword\")))"))
      (Ability|GameplayEffect|AddLooseGameplayTags self (GameplayTags|MakeLiteralGameplayTagContainer "(GameplayTags=((TagName=\"Character.Enemy\")))")))
    (:CastFailed
      (Development|PrintString "Hello"))))

(event EventUpdateState
  (params (New%20State :type E_EnemyState%20Enum :default "NewEnumerator0"))
  (bind _charactermovement (Variables|Character|GetCharacterMovement))
  (bind _output_get (Variables|Default|SetState New%20State))
  (switch Utilities|FlowControl|Switch|SwitchonE_EnemyState _output_get
    (:NewEnumerator0
      (Variables|/Script/Engine.CharacterMovementComponent|SetMaxWalkSpeed _charactermovement 6e+02))
    (:NewEnumerator1
      (Variables|/Script/Engine.CharacterMovementComponent|SetMaxWalkSpeed _charactermovement 2e+02))
    (:NewEnumerator2
      (Variables|/Script/Engine.CharacterMovementComponent|SetMaxWalkSpeed _charactermovement 2e+02))))

(event EventTick
  (params (DeltaSeconds :type Float%20%28single-precision%29))
  (bind _returnvalue (Game|Player|GetPlayerPawn 0))
  (Utilities|IsValid _returnvalue
    (:Is%20Valid
      (Transformation|SetWorldRotation (Variables|Default|GetHealth%20Bar%20Widget%20Component) (Math|Rotator|FindLookatRotation (Transformation|GetActorLocation) (Transformation|GetWorldLocation (Actor|GetComponentbyClass _returnvalue "/Script/Engine.CameraComponent"))) false false))))

(fn ConstructionScript)

(fn GiveAbilities
  (GameplayAbilities|GiveAbility (Variables|Default|GetAbilitySystemComponent) "/Game/GameplayAbilitySystem/Abilities/GA_EquipWeapon.GA_EquipWeapon_C" 0 -1)
  (GameplayAbilities|GiveAbility (Variables|Default|GetAbilitySystemComponent) "/Game/GameplayAbilitySystem/Abilities/GA_SwordAttack.GA_SwordAttack_C" 0 -1))