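; Base enemy character built on the Gameplay Ability System, exposing a behavior tree asset.
; BeginPlay initializes the health widget, grants sword abilities, sends an equip event, tags it as an enemy and sets the Manny anim Blueprint.
; Tick turns the health bar toward the player camera, while UpdateState sets walk speed per combat state.
; Flailing plays a falling montage and spins the mesh on a looping timer until stopped.
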(event Custom|StopFlailing
  ;[0.15 0.15 0.15 0.5] Flailing Behavior
  (Variables|Default|SetIsFlailing false)
  (Animation|StopAnimMontage "/Game/Animation/AM_Falling_Anim_Montage.AM_Falling_Anim_Montage")
  (Utilities|Time|ClearandInvalidateTimerbyHandle (stale Custom|StartFlailing _returnvalue))
  (Transformation|SetRelativeRotation (Variables|Character|GetMesh) (Math|Vector|RotatorfromAxisandAngle "0.000000,0.000000,1.000000" -9e+01) false false))

(event Custom|StartFlailing
  ;[0.15 0.15 0.15 0.5] Flailing Behavior
  (Variables|Default|SetIsFlailing true)
  (Animation|Montage|PlayMontage (Variables|Character|GetMesh) "/Game/Animation/AM_Falling_Anim_Montage.AM_Falling_Anim_Montage" 1.5 0.0 "Default"
    (:then
      (bind _returnvalue (Utilities|Time|SetTimerbyEvent (delegate Custom|Spin%20Character) 0.01 true true)))))

(event Custom|Spin%20Character
  ;[0.15 0.15 0.15 0.5] Flailing Behavior
  (Transformation|AddLocalRotation (Variables|Character|GetMesh) (Math|Vector|RotatorfromAxisandAngle "0.000000,0.000000,1.000000" 15.0) false false))

(event EventBeginPlay
  (bind _asw_enemy_health (Utilities|Casting|CastToW_EnemyHealth (UserInterface|GetWidget (Variables|Default|GetHealth%20Bar%20Widget%20Component)))
    (:then
      (Variables|/Game/UI/Widgets/W_EnemyHealth.W_EnemyHealth_C|SetOwning%20Enemy _asw_enemy_health self)
      (Default|Initialize _asw_enemy_health)
      (CallFunction|GiveAbilities)
      (Ability|SendGameplayEventtoActor self "(TagName=\"Event.Weapon.Equip\")" (Utilities|Struct|MakeGameplayEventData "(GameplayTags=((TagName=\"Weapon.Melee.Sword\")))"))
      (Ability|GameplayEffect|AddLooseGameplayTags self (GameplayTags|MakeLiteralGameplayTagContainer "(GameplayTags=((TagName=\"Character.Enemy\")))"))
      (Components|SkeletalMesh|SetAnimInstanceClass (Variables|Character|GetMesh) "/Game/SwordAnims/DEMO/Characters/Mannequins/Animations/ABP_Manny.ABP_Manny_C")
      (bind _asabp_manny (Utilities|Casting|CastToABP_Manny (Components|SkeletalMesh|GetAnimInstance (Variables|Character|GetMesh))))
      (Variables|/Game/SwordAnims/DEMO/Characters/Mannequins/Animations/ABP_Manny.ABP_Manny_C|SetArmSpace _asabp_manny (Variables|Default|GetABP%20Arm%20Space)))
    (:CastFailed
      (Development|PrintString "Hello"))))

(event EventUpdateState
  (params (New%20State :type E_EnemyState%20Enum :default "NewEnumerator0"))
  (bind _charactermovement (Variables|Character|GetCharacterMovement))
  (bind _output_get (Variables|Default|SetState New%20State))
  (switch Utilities|FlowControl|Switch|SwitchonE_EnemyState _output_get
    (:NewEnumerator0
      (Variables|/Script/Engine.CharacterMovementComponent|SetMaxWalkSpeed _charactermovement 6e+02))
    (:NewEnumerator1
      (Variables|/Script/Engine.CharacterMovementComponent|SetMaxWalkSpeed _charactermovement 2e+02))
    (:NewEnumerator2
      (Variables|/Script/Engine.CharacterMovementComponent|SetMaxWalkSpeed _charactermovement 3.5e+02))
    (:NewEnumerator3
      (Variables|/Script/Engine.CharacterMovementComponent|SetMaxWalkSpeed _charactermovement 1e+02))))

(event EventTick
  (params (DeltaSeconds :type Float%20%28single-precision%29))
  (bind _returnvalue (Game|Player|GetPlayerPawn 0))
  (Utilities|IsValid _returnvalue
    (:Is%20Valid
      (Transformation|SetWorldRotation (Variables|Default|GetHealth%20Bar%20Widget%20Component) (Math|Rotator|FindLookatRotation (Transformation|GetActorLocation) (Transformation|GetWorldLocation (Actor|GetComponentbyClass _returnvalue "/Script/Engine.CameraComponent"))) false false))))

(fn ConstructionScript)

(fn GiveAbilities
  (GameplayAbilities|GiveAbility (Variables|Default|GetAbilitySystemComponent) "/Game/GameplayAbilitySystem/Abilities/GA_EquipWeapon.GA_EquipWeapon_C" 0 -1)
  (GameplayAbilities|GiveAbility (Variables|Default|GetAbilitySystemComponent) "/Game/GameplayAbilitySystem/Abilities/GA_SwordAttack.GA_SwordAttack_C" 0 -1))

(fn GetBehaviorTreeAsset
  (return (Variables|Default|GetBehavior%20Tree%20Asset)))