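; BP_Projectile_Base is a base projectile actor that launches from its owner and reports overlaps with other actors.
; Launch sets move-ignores between projectile and owner, then feeds a direction to ProjectileMovement at fixed speed through SetVelocityInLocalSpace.
; Player-owned projectiles use the camera's forward vector, others the owner's forward vector.
; SphereCollision overlaps with non-owner actors call the projectile-connected dispatcher, with no hit effect applied here.
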(event OnComponentBeginOverlap(SphereCollision)
  (params (OverlappedComponent :type Primitive%20Component%20Object%20Reference) (OtherActor :type Actor%20Object%20Reference) (OtherComp :type Primitive%20Component%20Object%20Reference) (OtherBodyIndex :type Integer) (bFromSweep :type Boolean) (SweepResult :type Hit%20Result%20Structure%20%28by%20ref%29))
  (if (!= OtherActor (Components|GetOwner))
    (Default|CallProjectileConnectedDispatcher)))

(event Custom|Launch
  (CallFunction|SetupIgnore)
  (Utilities|IsValid (Components|GetOwner)
    (:Is%20Valid
      (CallFunction|InternalLaunch))))

(fn ConstructionScript)

(fn SetupIgnore
  (bind _returnvalue (Components|GetOwner))
  (Collision|IgnoreActorwhenMoving (Variables|Default|GetSphere%20Collision) _returnvalue true)
  (Collision|IgnoreActorwhenMoving (Actor|GetComponentbyClass _returnvalue "/Script/Engine.CapsuleComponent") self true)
  (Collision|IgnoreActorwhenMoving (Variables|Default|GetSphere) _returnvalue true))

(fn InternalLaunch
  (Utilities|FlowControl|Sequence
    (:then_0
      (if (CallFunction|IsOwnedbyPlayer)
        (LocalVariables|SetLaunch%20Direction (Math|Vector|GetForwardVector (Variables|/Script/Engine.PlayerCameraManager|GetTransformComponent (Game|GetPlayerCameraManager 0))))
        (else
          (LocalVariables|SetLaunch%20Direction (Transformation|GetActorForwardVector (Components|GetOwner))))))
    (:then_1
      (Game|Components|ProjectileMovement|SetVelocityinLocalSpace (Variables|Default|GetProjectileMovement) (* (LocalVariables|GetLaunch%20Direction) 2e+03)))))

(fn IsOwnedbyPlayer
  (Utilities|Casting|CastToBP_Player (Components|GetOwner)
    (:then
      (return true))
    (:CastFailed
      (return false))))