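; Gameplay ability that fires a fireball projectile from the avatar and deals area damage where it connects.
; Activation commits cost, spawns and launches BP_Projectile_Fireball, binds its hit dispatcher, commits cooldown and ends immediately.
; The later hit callback destroys the projectile, sphere-overlaps nearby pawns except the caster, and has each valid ability system component apply GE_ApplyDamage to itself.
; A gas-fire effect spawn is present but never runs.
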(event Custom|On%20Blast%20Hit
  (bind _output_get (Variables|Default|SetBlast%20Location (Transformation|GetActorLocation (stale Ability|EventActivateAbility _returnvalue_2))))
  (Actor|DestroyActor (stale Ability|EventActivateAbility _returnvalue_2))
  (bind (_outactors _returnvalue) (Collision|SphereOverlapActors _output_get 3e+02 (Utilities|Array|MakeArray "ObjectTypeQuery3") 0 (Utilities|Array|MakeArray (Ability|GetAvatarActorfromActorInfo))))
  (if _returnvalue
    (for _array_element _outactors
      (Utilities|IsValid (Ability|GetAbilitySystemComponent _array_element)
        (:Is%20Valid
          (GameplayEffects|ApplyGameplayEffectToSelf :self (Ability|GetAbilitySystemComponent _array_element) :GameplayEffectClass "/Game/GameplayAbilitySystem/Effects/GE_ApplyDamage.GE_ApplyDamage_C"))))))

(event Ability|EventActivateAbility
  (bind _returnvalue (Ability|GetAvatarActorfromActorInfo))
  (Ability|CommitAbilityCost false)
  (bind _returnvalue_2 (Game|SpawnActorfromClass "/Game/GameplayAbilitySystem/EffectActors/BP_Projectile_Fireball.BP_Projectile_Fireball_C" (Math|Transform|MakeTransform (Transformation|GetActorLocation _returnvalue) "0, 0, 0" "1.000000,1.000000,1.000000") "Undefined" "MultiplyWithRoot" _returnvalue 0))
  (Default|Launch _returnvalue_2)
  (EventDispatchers|BindEventtoProjectileConnectedDispatcher _returnvalue_2 (delegate Custom|On%20Blast%20Hit))
  (Ability|CommitAbilityCooldown false)
  (Ability|EndAbility))

(event Ability|EventOnEndAbility
  (params (bWasCancelled :type Boolean)))