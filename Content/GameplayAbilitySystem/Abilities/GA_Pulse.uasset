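; GA_Pulse is a gameplay ability that knocks nearby characters away from its avatar as temporary ragdolls.
; It commits cost and cooldown, sphere-overlaps pawns around the avatar, then ragdolls each CharacterBase and applies an outward velocity-change impulse scaled by PulsePower.
; After Duration it releases the same characters from ragdoll, adds the Water.Pulse gameplay cue set to remove on ability end, and immediately ends.
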(event Ability|EventActivateAbility
  (bind _returnvalue (Ability|GetAvatarActorfromActorInfo))
  (bind _returnvalue_2 (Transformation|GetActorLocation _returnvalue))
  (Ability|CommitAbilityCost false)
  (Ability|CommitAbilityCooldown false)
  (bind _outactors (Collision|SphereOverlapActors _returnvalue_2 3e+02 (Utilities|Array|MakeArray "ObjectTypeQuery3") 0 (Utilities|Array|MakeArray _returnvalue)))
  (Utilities|FlowControl|Sequence
    (:then_0
      (for _array_element _outactors
        (bind _ascharacter_base (Utilities|Casting|CastToCharacterBase _array_element))
        (CallFunction|Ragdoll _ascharacter_base true)
        (Physics|AddImpulse (Variables|/Script/Engine.Character|GetMesh _ascharacter_base) (* (Math|Vector|Normalize (- (Transformation|GetActorLocation _ascharacter_base) _returnvalue_2)) (Variables|Default|GetPulse%20Power)) "None" true)))
    (:then_1
      (Utilities|FlowControl|Delay (Variables|Default|GetDuration))
      (for _array_element_2 _outactors
        (bind _ascharacter_base_2 (Utilities|Casting|CastToCharacterBase _array_element_2))
        (CallFunction|Ragdoll _ascharacter_base_2 false))
      (GameplayCue|AddGameplayCue :GameplayCueTag "(TagName=\"GameplayCue.Water.Pulse\")")
      (Ability|EndAbility))))

(event Ability|EventOnEndAbility
  (params (bWasCancelled :type Boolean)))