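; Gameplay ability for the Hurricane spell, charged while input is held and cast on release.
; Activation hides the weapon, shows the hurricane orb, zooms the player camera in, plays an idle montage and adds a water gameplay cue.
; Release disables the crosshair and plays the attack montage, whose notify commits cost and cooldown, hides the orb and ends the ability.
; Montage completion triggers cleanup, restoring zoom and weapon visibility.
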(event Ability|EventActivateAbility
  (bind _returnvalue (Ability|GetAvatarActorfromActorInfo))
  (Utilities|IsValid _returnvalue
    (:Is%20Valid
      (bind _ascharacter_base (Utilities|Casting|CastToCharacterBase _returnvalue))
      (Variables|Default|SetCharacterBaseRef _ascharacter_base)
      (bind _characterbaseref (Variables|Default|GetCharacterBaseRef)
        (:then
          (CallFunction|Prepare)
          (Animation|Montage|PlayMontage (Variables|/Script/Engine.Character|GetMesh _characterbaseref) "/Game/Animation/AM_Standing_Idle_Anim.AM_Standing_Idle_Anim" 1.0 0.0 "Default"
            (:then
              (GameplayCue|AddGameplayCue :GameplayCueTag "(TagName=\"GameplayCue.Water.Hurricane\")")
              (Ability|Tasks|WaitInputRelease true
                (:OnRelease
                  (bind _asbp_third_person_player_controller (Utilities|Casting|CastToBP_ThirdPersonPlayerController (Game|GetPlayerController 0))
                    (:then
                      (Default|DisableCrosshair (Variables|/Game/ThirdPerson/Blueprints/BP_ThirdPersonPlayerController.BP_ThirdPersonPlayerController_C|GetHUDRef _asbp_third_person_player_controller)))
                    (:CastFailed
                      _))
                  (bind _notifyname (Animation|Montage|PlayMontage (Variables|/Script/Engine.Character|GetMesh _characterbaseref) "/Game/Animation/AM_Standing_2H_Magic_Attack_01_Montage.AM_Standing_2H_Magic_Attack_01_Montage")
                    (:OnCompleted
                      (CallFunction|Cleanup))
                    (:OnNotifyBegin
                      (switch name _notifyname
                        (:AMN_MagicRelease
                          (Ability|CommitAbilityCost false)
                          (Ability|CommitAbilityCooldown false)
                          (Rendering|SetVisibility (Variables|/Script/DrownMeNot.CharacterBase|GetHurricaneOrbMeshComponent (Variables|Default|GetCharacterBaseRef)) false true)
                          (Ability|EndAbility))))))))))
        (:else)))))

(fn Prepare
  (bind _characterbaseref (Variables|Default|GetCharacterBaseRef))
  (bind _returnvalue (Actor|GetComponentbyClass _characterbaseref "/Game/Weapons/BPC_WeaponsManager.BPC_WeaponsManager_C"))
  ;[0.15 0.15 0.15 0.5] HideWeaponIfValid
  (Utilities|IsValid _returnvalue
    (:Is%20Valid
      (bind _output_get (Variables|Default|SetEquipped%20Weapon (Variables|/Game/Weapons/BPC_WeaponsManager.BPC_WeaponsManager_C|GetEquipped%20Weapon _returnvalue)))
      (Rendering|ToggleVisibility (Variables|/Game/Weapons/BP_Weapon_Base.BP_Weapon_Base_C|GetWeapon%20Mesh _output_get) true)
      ;[0.15 0.15 0.15 0.5] Show Hurricane Orb
      (Rendering|SetVisibility (Variables|/Script/DrownMeNot.CharacterBase|GetHurricaneOrbMeshComponent (Variables|Default|GetCharacterBaseRef)) true true)
      (bind _asbp_player (Utilities|Casting|CastToBP_Player (Variables|Default|GetCharacterBaseRef)))
      (Utilities|IsValid _asbp_player
        (:Is%20Valid
          (Default|Zoomin _asbp_player)
          (return))))))

(fn Cleanup
  (bind _asbp_player (Utilities|Casting|CastToBP_Player (Variables|Default|GetCharacterBaseRef)))
  (Utilities|IsValid _asbp_player
    (:Is%20Valid
      (Default|ZoomOut _asbp_player))
    (:Is%20Not%20Valid
      _))
  (bind _equipped_weapon (Variables|Default|GetEquipped%20Weapon)
    (:then
      (Rendering|ToggleVisibility (Variables|/Game/Weapons/BP_Weapon_Base.BP_Weapon_Base_C|GetWeapon%20Mesh _equipped_weapon) true)
      (return))
    (:else)))