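; GA_FireSpray is a gameplay ability that deals damage with one forward spray from the avatar.
; On activation it adds the Water.WaterGun gameplay cue, runs Spray once and ends immediately, removing the cue.
; Spray sphere-traces pawns along the avatar's forward vector, ignoring all BP_Enemy_Base actors.
; The hit actor's ability system component, if valid, applies GE_ApplyDamage to itself.
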(event Custom|Spray
  (bind _returnvalue (Ability|GetAvatarActorfromActorInfo))
  (bind _returnvalue_2 (Transformation|GetActorLocation _returnvalue))
  (bind (_outhit _returnvalue_3) (Collision|SphereTraceForObjects _returnvalue_2 (+ _returnvalue_2 (* (Transformation|GetActorForwardVector _returnvalue) (Variables|Default|GetSpray%20Range))) (Variables|Default|GetRadius) (Utilities|Array|MakeArray "ObjectTypeQuery3") false (stale Ability|EventActivateAbility _outactors) "ForOneFrame"))
  ;[0.15 0.15 0.15 0.5] Must have hit pawn
  (if _returnvalue_3
    (Utilities|IsValid (Ability|GetAbilitySystemComponent (.HitActor (Collision|BreakHitResult _outhit)))
      (:Is%20Valid
        (GameplayEffects|ApplyGameplayEffectToSelf :self (Ability|GetAbilitySystemComponent (.HitActor (Collision|BreakHitResult _outhit))) :GameplayEffectClass "/Game/GameplayAbilitySystem/Effects/GE_ApplyDamage.GE_ApplyDamage_C")))))

(event Ability|EventActivateAbility
  (GameplayCue|AddGameplayCue :GameplayCueTag "(TagName=\"GameplayCue.Water.WaterGun\")")
  (bind _outactors (Actor|GetAllActorsOfClass "/Game/GameplayAbilitySystem/Characters/BP_Enemy_Base.BP_Enemy_Base_C"))
  (CallFunction|Spray)
  (Ability|EndAbility))