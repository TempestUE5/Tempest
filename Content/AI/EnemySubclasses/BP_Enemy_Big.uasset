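; BP_Enemy_Big is a big enemy subclass that carries a fire spray ability and a 300-point health pool.
; On BeginPlay it runs the parent logic, then has WeaponsManager unequip its weapon.
; It extends the parent's GiveAbilities to grant GA_FireSpray through the Ability System Component, then raises or sets max health and restores it to full.
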(event EventBeginPlay
  (|CallParentFunction)
  (Default|UnequipWeapon (Variables|Default|GetWeapons%20Manager)))

(event Collision|EventActorBeginOverlap
  (params (OtherActor :type Actor%20Object%20Reference)))

(event EventTick
  (params (DeltaSeconds :type Float%20%28single-precision%29))
  (|CallParentFunction DeltaSeconds) ; This node is disabled and will not be called.\nDrag off pins to build functionality.
)

(fn ConstructionScript
  (|CallParentFunction))

(fn GiveAbilities
  (|CallParentFunction)
  (GameplayAbilities|GiveAbility (Variables|Default|GetAbilitySystemComponent) "/Game/GameplayAbilitySystem/Abilities/GA_FireSpray.GA_FireSpray_C" 0 -1)
  (Class|CharacterBase|SetMaxHealth 3e+02)
  (Class|CharacterBase|RestoreHealthtoFull))