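; Hurricane ability actor that is aimed, launched and pulls in nearby enemies while its Niagara effect is active.
; A looping timer predicts its trajectory toward the mouse target for the player, or a seeded random target for other casters, until launch.
; Box overlaps track enemies, and Tick applies outer attraction or inner pull, lift and flailing by horizontal distance.
; Debug boxes show both radii, and effect completion clears affected enemies.
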(event OnComponentBeginOverlap(BoxCollision)
  (params (OverlappedComponent :type Primitive%20Component%20Object%20Reference) (OtherActor :type Actor%20Object%20Reference) (OtherComp :type Primitive%20Component%20Object%20Reference) (OtherBodyIndex :type Integer) (bFromSweep :type Boolean) (SweepResult :type Hit%20Result%20Structure%20%28by%20ref%29))
  ;[0.15 0.15 0.15 0.5] ADD TO ENEMY SET
  (bind _asbp_enemy_base (Utilities|Casting|CastToBP_Enemy_Base OtherActor))
  (Utilities|IsValid _asbp_enemy_base
    (:Is%20Valid
      (Utilities|Set|Add (Variables|Physics|GetOverlappingEnemies) _asbp_enemy_base))))

(event OnComponentEndOverlap(BoxCollision)
  (params (OverlappedComponent :type Primitive%20Component%20Object%20Reference) (OtherActor :type Actor%20Object%20Reference) (OtherComp :type Primitive%20Component%20Object%20Reference) (OtherBodyIndex :type Integer))
  ;[0.15 0.15 0.15 0.5] REMOVE FROM ENEMY SET
  (bind _asbp_enemy_base (Utilities|Casting|CastToBP_Enemy_Base OtherActor))
  (Utilities|Set|Remove (Variables|Physics|GetOverlappingEnemies) _asbp_enemy_base)
  (if (Variables|/Game/GameplayAbilitySystem/Characters/BP_Enemy_Base.BP_Enemy_Base_C|GetIsFlailing _asbp_enemy_base)
    (Default|StopFlailing _asbp_enemy_base)))

(event OnSystemFinished(NS_HurricaneComponent)
  (params (PSystem :type Niagara%20Component%20Object%20Reference))
  (bind _overlappingenemies (Variables|Physics|GetOverlappingEnemies))
  (if (Utilities|Set|IsNotEmpty _overlappingenemies)
    (bind _result (Utilities|Set|ToArray _overlappingenemies))
    (for _array_element _result
      (if (Variables|/Game/GameplayAbilitySystem/Characters/BP_Enemy_Base.BP_Enemy_Base_C|GetIsFlailing _array_element)
        (Default|StopFlailing _array_element)
        (Pawn|Components|CharacterMovement|ClearAccumulatedForces (Variables|/Script/Engine.Character|GetCharacterMovement _array_element))))
    (Utilities|Set|Clear _overlappingenemies)
    (Development|PrintString "cleared")))

(event Custom|PredictTrajectory
  (params (CharacterRef :type Character%20Base%20Object%20Reference))
  (bind _playerhudref (Variables|Default|GetPlayerHUDRef))
  (Variables|Default|SetTimeDispatched (Math|Float|Floor (Utilities|Time|GetGameTimeinSeconds)))
  (Utilities|IsValid _playerhudref
    (:Is%20Valid
      (Default|EnableCrosshair _playerhudref))
    (:Is%20Not%20Valid
      _))
  (bind _returnvalue (Utilities|Time|SetTimerbyEvent (delegate Custom|UpdateTrajectory) 0.01 true)))

(event Custom|LaunchHurricane
  (Utilities|Time|ClearandInvalidateTimerbyHandle (stale Custom|PredictTrajectory _returnvalue))
  (Class|Hurricane|TriggerLaunchHurricane))

(event Custom|UpdateTrajectory
  (Render|ComputeHurricaneTrajectory (stale Custom|PredictTrajectory CharacterRef)))

(event EventBeginPlay
  (bind _asbp_third_person_player_controller (Utilities|Casting|CastToBP_ThirdPersonPlayerController (Game|GetPlayerController 0)))
  (Variables|Default|SetPlayerHUDRef (Variables|/Game/ThirdPerson/Blueprints/BP_ThirdPersonPlayerController.BP_ThirdPersonPlayerController_C|GetHUDRef _asbp_third_person_player_controller)))

(event EventTick
  (params (DeltaSeconds :type Float%20%28single-precision%29))
  (bind _ns_hurricanecomponent (Variables|Default|GetNS_HurricaneComponent))
  (bind _boxcollision (Variables|Default|GetBoxCollision))
  (bind _outersearchradius (Variables|Physics|GetOuterSearchRadius))
  (bind _boxcollision_2 (Variables|Default|GetBoxCollision))
  (bind _innersearchradius (Variables|Physics|GetInnerSearchRadius))
  (bind _returnvalue (Components|Activation|IsActive _ns_hurricanecomponent))
  (bind _returnvalue_2 (Transformation|GetWorldLocation _boxcollision))
  (bind _returnvalue_3 (Components|Box|GetUnscaledBoxExtent _boxcollision_2))
  ;[0.15 0.15 0.15 0.5] TICK WHEN ACTIVE AND OVERLAPS FOUND
  (Utilities|FlowControl|Sequence
    (:then_0
      (if (and (Utilities|Set|IsNotEmpty (Variables|Physics|GetOverlappingEnemies)) _returnvalue)
        (Physics|AffectEnemies)))
    (:then_1
      ;[0.15 0.15 0.15 0.5] DEBUG BOXES
      (if _returnvalue
        (Rendering|Debug|DrawDebugBox _returnvalue_2 (Math|Vector|MakeVector _innersearchradius _innersearchradius (.z _returnvalue_3)) "(R=1.000000,G=0.184243,B=0.000000,A=1.000000)" "0, 0, 0" 0.0 1e+01)
        (Rendering|Debug|DrawDebugBox _returnvalue_2 (Math|Vector|MakeVector _outersearchradius _outersearchradius (.z _returnvalue_3)) "(R=1.000000,G=0.000000,B=0.213178,A=1.000000)" "0, 0, 0" 0.0 1e+01)))))

(fn ConstructionScript
  (bind _outersearchradius (Variables|Physics|GetOuterSearchRadius))
  (Class|Hurricane|SetAnimationDuration (Variables|Default|GetAnimationDuration))
  (Components|Box|SetBoxExtent (Variables|Default|GetBoxCollision) (Math|Vector|MakeVector _outersearchradius _outersearchradius (.z (Components|Box|GetUnscaledBoxExtent (Variables|Default|GetBoxCollision)))) true))

(fn ComputeHurricaneTrajectory
  (params (CharacterRef :type Character%20Base%20Object%20Reference))
  (bind _asbp_player (Utilities|Casting|CastToBP_Player CharacterRef))
  (Utilities|IsValid _asbp_player
    (:Is%20Valid
      (bind _worldlocation (Render|ComputeMouseTarget 1e+03))
      (LocalVariables|SetTargetPos _worldlocation))
    (:Is%20Not%20Valid
      (bind _out (Render|ComputeRandomTarget CharacterRef 1.5e+03))
      (LocalVariables|SetTargetPos _out)))
  (Class|Hurricane|PredictHurricaneTrajectory (.Location (Math|Transform|BreakTransform (Transformation|GetSocketTransform (Variables|/Script/Engine.Character|GetMesh CharacterRef) "HurricaneStartSocket" "RTS_World"))) (LocalVariables|GetTargetPos) (Transformation|GetActorForwardVector CharacterRef) 0.1)
  (return))

(fn ComputeMouseTarget
  (params (Magnitude :type Float%20%28double-precision%29))
  (bind _returnvalue (Game|GetPlayerController 0))
  (bind _playerhudref (Variables|Default|GetPlayerHUDRef))
  (bind (_worldlocation _worlddirection) (Game|Player|ConvertMouseLocationToWorldSpace _returnvalue))
  (bind _returnvalue_2 (* Magnitude _worlddirection))
  (bind _returnvalue_3 (+ _worldlocation _returnvalue_2))
  (bind _screenposition (Class|GameplayStatics|ProjectWorldtoScreen _returnvalue _returnvalue_3 false))
  (bind (_x _y) (Math|Vector2D|BreakVector2D _screenposition))
  (Utilities|IsValid _playerhudref
    (:Is%20Valid
      (Default|UpdateCrosshair _playerhudref _x _y))
    (:Is%20Not%20Valid
      _))
  (return _returnvalue_3))

(fn ComputeRandomTarget
  (params (CharacterRef :type Character%20Base%20Object%20Reference) (Magnitude :type Float%20%28double-precision%29))
  (bind _returnvalue (Utilities|GetObjectName CharacterRef))
  (bind _timedispatched (Variables|Default|GetTimeDispatched))
  (bind _returnvalue_2 (Math|Conversions|ToInteger(Byte) _returnvalue))
  (bind _returnvalue_3 (+ _returnvalue_2 _timedispatched))
  (bind _returnvalue_4 (Math|Random|MakeRandomStream _returnvalue_3))
  (return (+ (Transformation|GetActorLocation CharacterRef) (* Magnitude (Math|Vector|Normalize (Math|Vector|MakeVector (Math|Random|RandomFloatinRangefromStream _returnvalue_4 -1.0 1.0) (Math|Random|RandomFloatinRangefromStream _returnvalue_4 -1.0 1.0) 0.0))))))

(fn AffectEnemies
  (bind _result (Utilities|Set|ToArray (Variables|Physics|GetOverlappingEnemies)))
  (for _array_element _result
    (if (< (Math|Vector|VectorLength (- (Math|Vector|ProjectVectorontoPlane (Transformation|GetActorLocation) "0.000000,0.000000,1.000000") (Math|Vector|ProjectVectorontoPlane (Transformation|GetActorLocation _array_element) "0.000000,0.000000,1.000000"))) (Variables|Physics|GetInnerSearchRadius))
      (Physics|DoInnerEffect (- (Math|Vector|ProjectVectorontoPlane (Transformation|GetActorLocation) "0.000000,0.000000,1.000000") (Math|Vector|ProjectVectorontoPlane (Transformation|GetActorLocation _array_element) "0.000000,0.000000,1.000000")) _array_element (Math|Vector|VectorLength (- (Math|Vector|ProjectVectorontoPlane (Transformation|GetActorLocation) "0.000000,0.000000,1.000000") (Math|Vector|ProjectVectorontoPlane (Transformation|GetActorLocation _array_element) "0.000000,0.000000,1.000000"))))
      (else
        (Physics|DoOuterEffect (- (Math|Vector|ProjectVectorontoPlane (Transformation|GetActorLocation) "0.000000,0.000000,1.000000") (Math|Vector|ProjectVectorontoPlane (Transformation|GetActorLocation _array_element) "0.000000,0.000000,1.000000")) _array_element)))
    (return)))

(fn DoOuterEffect
  (params (EnemyToHurricane :type Vector) (EnemyRef :type BP%20Enemy%20Base%20Object%20Reference))
  (Physics|AddImpulse (Variables|/Script/Engine.Character|GetCharacterMovement EnemyRef) (* (* (Variables|Physics|GetOuterAttractionScalar) (Math|Float|MapRangeClamped (Math|Vector|VectorLength EnemyToHurricane) (Variables|Physics|GetInnerSearchRadius) (Variables|Physics|GetOuterSearchRadius) 1.0 0.0)) (Math|Vector|Normalize (+ EnemyToHurricane "0.000000,0.000000,250.000000"))) false)
  (if (Variables|/Game/GameplayAbilitySystem/Characters/BP_Enemy_Base.BP_Enemy_Base_C|GetIsFlailing EnemyRef)
    (Default|StopFlailing EnemyRef)))

(fn DoInnerEffect
  (params (EnemyToHurricane :type Vector) (EnemyRef :type BP%20Enemy%20Base%20Object%20Reference) (EnemyRadius :type Float%20%28double-precision%29))
  (bind _charactermovement (Variables|/Script/Engine.Character|GetCharacterMovement EnemyRef))
  (Physics|AddImpulse _charactermovement (* (Variables|Physics|GetInnerAttractionScalar) (Math|Vector|Normalize (Math|Vector|ProjectVectorontoPlane EnemyToHurricane "0.000000,0.000000,1.000000"))) false)
  (if (< (.z (Transformation|GetActorLocation EnemyRef)) (+ (.z (Transformation|GetWorldLocation (Variables|Default|GetBoxCollision))) 0.0))
    (Physics|AddImpulse _charactermovement "0.000000,0.000000,3000.000000" false)
    (else
      (Development|PrintString "Hello")))
  (if (not (Variables|/Game/GameplayAbilitySystem/Characters/BP_Enemy_Base.BP_Enemy_Base_C|GetIsFlailing EnemyRef))
    (Default|StartFlailing EnemyRef)
    (Transformation|SetWorldRotation (Variables|/Script/Engine.Character|GetMesh EnemyRef) (Math|Rotator|MakeRotator 0.0 0.0 0.0) false false)))